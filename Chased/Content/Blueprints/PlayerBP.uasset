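; Player character Blueprint with yaw-relative movement, mouse look, input-scaled camera-shake bob and a stamina-limited sprint.
; Axis input sets IsMoving and the Run action sets ShiftPressed; PlayerRunning combines them with stamina checks.
; Tick switches walk speed, drains or regenerates clamped stamina through helper functions, and prints it on screen.
; CanRun updates only while not running, so sprint re-entry requires stamina above a separate breakpoint.
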(event EventTick
  (params (DeltaSeconds :type Float%20%28single-precision%29))
  (bind _charactermovement (Variables|Character|GetCharacterMovement))
  ;[1 1 1] Stamina system
  (bind _output_get (Variables|Default|SetDTime DeltaSeconds))
  (Development|PrintString (Utilities|String|ToString(Float) (Variables|Default|GetStamina)) true true "(R=0.000000,G=0.660000,B=1.000000,A=1.000000)" _output_get)
  (bind _isrunning (CallFunction|PlayerRunning))
  (if _isrunning
    (Variables|/Script/Engine.CharacterMovementComponent|SetMaxWalkSpeed _charactermovement (Variables|Default|GetRunSpeed))
    (bind _returnvalue (CallFunction|ReduceStamina))
    (Variables|Default|SetStamina _returnvalue)
    (else
      (Variables|/Script/Engine.CharacterMovementComponent|SetMaxWalkSpeed _charactermovement 6e+02)
      (bind _returnvalue_2 (CallFunction|RegenStamina))
      (Variables|Default|SetStamina _returnvalue_2)
      (Variables|Default|SetCanRun (> (Variables|Default|GetStamina) (Variables|Default|GetStaminaRunBreakpoint))))))

(event Input|ActionEvents|InputActionRun
  (params (Key :type Key%20Structure))
  ;[1 1 1] Stamina system
  ;;[1 1 1] ShiftPressed
  (:Pressed
    (Variables|Default|SetShiftPressed true))
  (:Released
    (Variables|Default|SetShiftPressed false)))

(event Input|AxisEvents|InputAxisVertical
  (params (AxisValue :type Float%20%28single-precision%29))
  ;[1 1 1] Movement
  (Pawn|Input|AddMovementInput (Math|Vector|GetForwardVector (Math|Rotator|MakeRotator 0.0 0.0 (.Yaw (Math|Rotator|BreakRotator (Pawn|GetControlRotation :!class /Script/Engine.Pawn))))) AxisValue false)
  (Class|PlayerController|ClientPlayCameraShake (Game|GetPlayerController 0) "/Game/Blueprints/CameraBob.CameraBob_C" (Math|Float|Absolute(Float) AxisValue) "CameraLocal" "0, 0, 0"))

(event Input|AxisEvents|InputAxisHorizontal
  (params (AxisValue :type Float%20%28single-precision%29))
  ;[1 1 1] Movement
  (Pawn|Input|AddMovementInput (Math|Vector|GetRightVector (Math|Rotator|MakeRotator 0.0 0.0 (.Yaw (Math|Rotator|BreakRotator (Pawn|GetControlRotation :!class /Script/Engine.Pawn))))) AxisValue false)
  (Class|PlayerController|ClientPlayCameraShake (Game|GetPlayerController 0) "/Game/Blueprints/CameraBob.CameraBob_C" (Math|Float|Absolute(Float) AxisValue) "CameraLocal" "0, 0, 0"))

(event Input|AxisEvents|InputAxisVertical
  (params (AxisValue :type Float%20%28single-precision%29))
  ;[1 1 1] Stamina system
  ;;[1 1 1] IsMoving
  (Variables|Default|SetIsMoving (!= (Math|Conversions|ToFloat(Integer) (Class|KismetMathLibrary|OrIntInt (Math|Float|Truncate AxisValue) (Math|Float|Truncate (stale Input|AxisEvents|InputAxisHorizontal AxisValue)))) 0.0)))

(event Input|AxisEvents|InputAxisHorizontal
  (params (AxisValue :type Float%20%28single-precision%29))
  ;[1 1 1] Stamina system
  ;;[1 1 1] IsMoving
  (Variables|Default|SetIsMoving (!= (Math|Conversions|ToFloat(Integer) (Class|KismetMathLibrary|OrIntInt (Math|Float|Truncate (stale Input|AxisEvents|InputAxisVertical AxisValue)) (Math|Float|Truncate AxisValue))) 0.0)))

(event Input|AxisEvents|InputAxisMouseX
  (params (AxisValue :type Float%20%28single-precision%29))
  ;[1 1 1] Camera control
  (Pawn|Input|AddControllerYawInput AxisValue))

(event Input|AxisEvents|InputAxisMouseY
  (params (AxisValue :type Float%20%28single-precision%29))
  ;[1 1 1] Camera control
  (Pawn|Input|AddControllerPitchInput AxisValue))

(fn ConstructionScript)

(fn PlayerRunning
  (bind _output_get (Variables|Default|SetIsRunning (Math|Conversions|ToBoolean(Integer) (Class|KismetMathLibrary|AndIntInt (Math|Conversions|ToInteger(Boolean) (Variables|Default|GetShiftPressed)) (Math|Conversions|ToInteger(Boolean) (Variables|Default|GetIsMoving)) (Math|Conversions|ToInteger(Boolean) (> (Variables|Default|GetStamina) 2e+01)) (Math|Conversions|ToInteger(Boolean) (Variables|Default|GetCanRun))))))
  (return _output_get))

(fn ReduceStamina
  (return (Math|Float|Clamp(Float) (- (Variables|Default|GetStamina) (* (Variables|Default|GetDTime) (Variables|Default|GetStaminaDecreaseRate))) 0.0 (Variables|Default|GetMaxStamina))))

(fn RegenStamina
  (return (Math|Float|Clamp(Float) (+ (* (Variables|Default|GetDTime) (Variables|Default|GetStaminaRegenRate)) (Variables|Default|GetStamina)) 0.0 (Variables|Default|GetMaxStamina))))